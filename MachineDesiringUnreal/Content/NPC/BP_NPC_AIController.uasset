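; AI controller that drives Mover-based NPC pawns through wandering, gaze targeting and perception, with heavy debug drawing.
; Execute events start self-repeating AIMoveTo loops: long-range random walks (also used for idle and mating) or short crouched target walks.
; Gaze events set or clear the pawn's target, while a looping timer halts and restarts walking when the gaze-walk dot is negative.
; Sight updates report sensed or lost NPCs by their brain component ID.
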(event `RandomWalk`
  (bind _my_movertest (`self.MY_MOVERTEST`))
  (bind _returnvalue (`self.K2_GetActorLocation` _my_movertest))
  (bind _randomlocation (`NavigationSystemV1.K2_GetRandomReachablePointInRadius` _returnvalue 30000.0 null null))
  (if (not true)
    (`KismetSystemLibrary.DrawDebugBox` _returnvalue (100.0 100.0 100.0) (struct) (struct) 5.0 5.0)
    (`KismetSystemLibrary.DrawDebugLine` _returnvalue _randomlocation (struct :`G` 0.210231 :`B` 1.0 :`A` 1.0) 5.0 5.0)
    (`KismetSystemLibrary.DrawDebugBox` _randomlocation (100.0 100.0 100.0) (struct :`G` 0.02103 :`B` 1.0 :`A` 1.0) (struct) 5.0 5.0))
  (`|AIMoveTo` _my_movertest _randomlocation null 150.0
    (:`OnSuccess`
      (`KismetSystemLibrary.DrawDebugSphere` _randomlocation 20.0 12 (struct :`G` 1.0 :`B` 0.036887 :`A` 1.0) 5.0 5.0))
    (:`OnFail`
      (`KismetSystemLibrary.DrawDebugSphere` _randomlocation 20.0 12 (struct :`R` 1.0 :`G` 0.0492 :`B` 0.000186 :`A` 1.0) 5.0 5.0)))
  (`KismetSystemLibrary.Delay` 2.5)
  (`self.RandomWalk`))

(event `self.ReceivePossess`
  (params (PossessedPawn :type "Pawn Object Reference"))
  (set `self.My Desired Rank` (`_npcBrainComponent.myDesiredRank` (`self.GetComponentByClass` PossessedPawn "/Script/MachineDesiring._npcBrainComponent")))
  (bind _asmy_movertest (cast `/Game/NPC/MY_MOVERTEST` (`self.K2_GetPawn`)))
  (set `self.MY_MOVERTEST` _asmy_movertest))

(event `self.ReceiveBeginPlay`
  (`KismetSystemLibrary.K2_SetTimerDelegate` (delegate `checkgaze`) 0.5 true))

(event `checkgaze`
  (bind _mygazewalkdot (`self.myGazeWalkDot`))
  (if (< _mygazewalkdot 0.0)
    (`KismetSystemLibrary.PrintString` (`KismetStringLibrary.Conv_DoubleToString` _mygazewalkdot))
    (`self.StopMovement`)
    (`KismetSystemLibrary.Delay` 2.0)
    (`self.RandomWalk`)))

(event `self.BP_ExecuteMatingWait`
  (params (Location :type "Vector Structure") (Duration :type "Float (single-precision)") (BaseYaw :type "Float (single-precision)") (PhaseOffset :type "Float (single-precision)"))
  (`self.RandomWalk` :!label _label))

(event `TargetWalk`
  (bind _my_movertest (`self.MY_MOVERTEST`))
  (bind _randomlocation (`NavigationSystemV1.K2_GetRandomReachablePointInRadius` (`self.K2_GetActorLocation` _my_movertest) 900.0 null null))
  (`CharacterMoverComponent.Crouch` (`/Game/NPC/SandboxCharacter_Mover.CharacterMover` (`self.MY_MOVERTEST`)))
  (`|AIMoveTo` _my_movertest _randomlocation null
    (:`OnSuccess`
      (`KismetSystemLibrary.DrawDebugSphere` _randomlocation 100.0 12 (struct :`R` 1.0 :`G` 0.062795 :`B` 0.635935 :`A` 1.0) 5.0 5.0)
      (`KismetSystemLibrary.Delay` 2.0)
      (`self.TargetWalk`))))

(event `self.BP_ExecuteMatingMove`
  (params (Destination :type "Vector Structure"))
  (goto _label))

(event `self.BP_ExecuteRandomWalk`
  (params (Destination :type "Vector Structure"))
  (`KismetSystemLibrary.Delay` 0.2)
  (goto _label))

(event `self.BP_ExecuteIdleWait`
  (params (Location :type "Vector Structure") (Duration :type "Float (single-precision)") (BaseYaw :type "Float (single-precision)") (PhaseOffset :type "Float (single-precision)"))
  (goto _label))

(event `self.BP_ExecuteTargetWalk`
  (params (Destination :type "Vector Structure") (SpeedMult :type "Float (single-precision)") (TargetId :type Integer))
  (`self.TargetWalk`))

(event `self.ReceiveTick`
  (params (DeltaSeconds :type "Float (single-precision)"))
  (bind _my_movertest (`self.MY_MOVERTEST`))
  (bind _targetedactor (`/Game/NPC/SandboxCharacter_Mover.TargetedActor` _my_movertest))
  (if (`KismetSystemLibrary.IsValid` _targetedactor)
    (`KismetSystemLibrary.DrawDebugLine` (`self.K2_GetActorLocation` _my_movertest) (`self.K2_GetActorLocation` _targetedactor) (struct :`R` 1.0 :`B` 0.392397 :`A` 1.0) 0.0 1.0)))

(event `Idle`
  (`CharacterMoverComponent.Jump` (`/Game/NPC/SandboxCharacter_Mover.CharacterMover` (`self.MY_MOVERTEST`)))
  (`KismetSystemLibrary.Delay` 1.5)
  (`self.Idle`))

(event `Mating`
  (`CharacterMoverComponent.Crouch` (`/Game/NPC/SandboxCharacter_Mover.CharacterMover` (`self.MY_MOVERTEST`))))

(event `self.BP_ExecuteGazeLookAt`
  (params (TargetPawn :type "Pawn Object Reference"))
  (`KismetSystemLibrary.DrawDebugBox` (`self.K2_GetActorLocation` TargetPawn) (20.0 20.0 20.0) (struct :`R` 0.940735 :`G` 1.0 :`A` 1.0) (struct) 0.5 1.0)
  (set `/Game/NPC/SandboxCharacter_Mover.TargetedActor` TargetPawn (`self.MY_MOVERTEST`))
  (for _array_element (`self.My Desired Rank`)
    (`KismetSystemLibrary.PrintString` (`KismetStringLibrary.Conv_IntToString` _array_element))))

(event `self.BP_ClearGaze`
  (set `self.Target Pawn` null)
  (set `/Game/NPC/SandboxCharacter_Mover.TargetedActor` null (`self.MY_MOVERTEST`)))

(event `self.AIPerception.OnTargetPerceptionUpdated`
  (params (Actor :type "Actor Object Reference") (Stimulus :type "AIStimulus Structure"))
  (bind _returnvalue (`self.GetComponentByClass` Actor "/Script/MachineDesiring._npcBrainComponent"))
  (bind _myid (`_npcBrainComponent.myId` _returnvalue))
  (if Stimulus_bSuccessfullySensed
    (`/Engine/EditorBlueprintResources/StandardMacros.IsValid` _returnvalue
      (:`Is Valid`
        (`self.OnNearbyNPCsUpdated` (`|MakeArray` _myid))))
    (else
      (`/Engine/EditorBlueprintResources/StandardMacros.IsValid` _returnvalue
        (:`Is Valid`
          (`self.OnNpcLostFromSight` _myid))))))

(event `self.AIPerception.OnPerceptionUpdated`
  (params (UpdatedActors :type "Array of Actor Object Reference (by ref)")))

(fn `UserConstructionScript`)